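; Player-controllable tank Blueprint that drives on two tracks, aims a turret and barrel, and fires.
; On BeginPlay it wires the barrel and turret into TankAim, the tracks into TankMovement, and its Health into a HealthBar widget.
; Input feeds scaled movement intents and fire requests to those components, rotates an azimuth pivot and spring arm to aim, and toggles first- and third-person cameras.
; The construction script enables rigid-body collision notifications on both tracks.
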(event `self.ReceiveBeginPlay`
  (`TankAimComponent.Initialize` (`self.TankAim`) (`self.TankBarrel`) (`self.TankTurret`))
  (`TankMovementComponent.Initialize` (`self.TankMovement`) (`self.Left_Track`) (`self.Right_Track`))
  (`self.InitializeHealthBarWidget`))

(event `InputAction|SwapCam`
  (params (Key :type "Key Structure"))
  (:`Pressed`
    (`ActorComponent.ToggleActive` (`self.TpsCamera`))
    (`ActorComponent.ToggleActive` (`self.FpsCamera`))))

(event `InputAxis|MoveForward`
  (params (AxisValue :type "Float (single-precision)"))
  (`TankMovementComponent.IntendMoveForward` (`self.TankMovement`) (* AxisValue 100.0)))

(event `InputAxis|AimAzimuth`
  (params (AxisValue :type "Float (single-precision)"))
  (`SceneComponent.K2_AddLocalRotation` (`self.Azimuth`) (`KismetMathLibrary.MakeRotator` 0.0 0.0 (* AxisValue (`GameplayStatics.GetWorldDeltaSeconds`) 100.0)) false false))

(event `InputAxis|TurnRight`
  (params (AxisValue :type "Float (single-precision)"))
  (`TankMovementComponent.IntendMoveRight` (`self.TankMovement`) (* AxisValue 250.0)))

(event `InputAxis|AimElevation`
  (params (AxisValue :type "Float (single-precision)"))
  (`SceneComponent.K2_AddLocalRotation` (`self.SpringArm`) (`KismetMathLibrary.MakeRotator` 0.0 (* AxisValue (`GameplayStatics.GetWorldDeltaSeconds`) 100.0)) false false))

(event `InputAction|Fire`
  (params (Key :type "Key Structure"))
  (:`Pressed`
    (`TankAimComponent.Fire` (`self.TankAim`))))

(fn `InitializeHealthBarWidget`
  (bind _ashealth_bar (cast `/Game/UI/HealthBar` (`WidgetComponent.GetUserWidgetObject` (`self.Widget`))))
  (set `/Game/UI/HealthBar.HealthReference` (`self.Health`) _ashealth_bar)
  (set `/Game/UI/HealthBar.TankReference` self _ashealth_bar)
  (return))

(fn `UserConstructionScript`
  (`PrimitiveComponent.SetNotifyRigidBodyCollision` (`self.Left_Track`) true)
  (`PrimitiveComponent.SetNotifyRigidBodyCollision` (`self.Right_Track`) true))